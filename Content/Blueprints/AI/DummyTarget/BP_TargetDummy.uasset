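; BP_TargetDummy is a target dummy that displays the damage it takes, both per hit and as a running total.
; BeginPlay creates two widgets and assigns them to its widget components.
; AnyDamage adds to the total and sends both values through server-then-multicast events to the widgets.
; A non-retriggerable five-second Delay clears the accumulated value, timed from the first hit rather than the last, without refreshing the displayed text.
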(event Custom|Multicast_SetTotalDamageText
  (params (DamageText :type Text))
  (Default|ServerSetTotalDamageText (Variables|Default|GetTotalDamage) DamageText))

(event Custom|Multicast_SetDamageText
  (params (DamageText :type Text))
  (Default|ServerSetDamageText (Variables|Default|GetDamage) DamageText))

(event Custom|Server_SetDamageText
  (params (DamageText :type Text))
  (CallFunction|MulticastSetDamageText DamageText))

(event Custom|Server_SetTotalDamageText
  (params (DamageText :type Text))
  (CallFunction|MulticastSetTotalDamageText DamageText))

(event Game|Damage|EventAnyDamage
  (params (Damage :type Float%20%28single-precision%29) (DamageType :type Damage%20Type%20Object%20Reference) (InstigatedBy :type Controller%20Object%20Reference) (DamageCauser :type Actor%20Object%20Reference))
  (Utilities|FlowControl|Sequence
    (:then_0
      (bind _output_get (Variables|Default|SetAccumulated%20damage (+ (Variables|Default|GetAccumulated%20damage) Damage)))
      (CallFunction|ServerSetTotalDamageText (Utilities|Text|FormatText "{.f}" _output_get))
      (Utilities|FlowControl|Delay 5.0)
      (Variables|Default|SetAccumulated%20damage 0.0))
    (:then_1
      (CallFunction|ServerSetDamageText (Utilities|Text|FormatText "{.f}" Damage)))))

(event EventBeginPlay
  (Utilities|FlowControl|Sequence
    (:then_0
      (bind _returnvalue (UserInterface|CreateWidget "/Game/Blueprints/HUD/WBP_TotalDamageWidget.WBP_TotalDamageWidget_C"))
      (bind _output_get (Variables|Default|SetTotalDamage _returnvalue))
      (UserInterface|SetWidget (Variables|Default|GetTotalDamageWidget) _output_get))
    (:then_1
      (bind _returnvalue_2 (UserInterface|CreateWidget "/Game/Blueprints/HUD/WBP_DamageWidget.WBP_DamageWidget_C"))
      (bind _output_get_2 (Variables|Default|SetDamage _returnvalue_2))
      (UserInterface|SetWidget (Variables|Default|GetDamageWidget) _output_get_2))))

(fn ConstructionScript)