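; BP_AdvancedAI is an AI bot that runs the BT_AdvancedAI behavior tree and can be armed with several weapon types.
; On BeginPlay it starts the tree on its AI controller and increments the spawned bot count in BP_CoopGameMode, which it decrements when destroyed.
; Separate equip events for shotgun, sniper, grenade and rocket spawn the default weapon class at the bot and pass it to its Combat component.
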(event Custom|EquipShotgun
  (bind _defaultshotgun (Variables|Default|GetDefaultShotGun))
  (bind _combat (Variables|Default|GetCombat))
  (if (Utilities|IsValidClass _defaultshotgun)
    (bind _returnvalue (Game|SpawnActorfromClass _defaultshotgun (Math|Conversions|ToTransform(Vector) (Transformation|GetActorLocation)) "AlwaysSpawn" "MultiplyWithRoot" 0 0))
    (Utilities|IsValid _combat
      (:Is%20Valid
        (Class|CombatComponent|EquipWeapon _combat _returnvalue)))))

(event Custom|EquipRocket
  (bind _combat (Variables|Default|GetCombat))
  (bind _defaultrocket (Variables|Default|GetDefaultRocket))
  (if (Utilities|IsValidClass _defaultrocket)
    (bind _returnvalue (Game|SpawnActorfromClass _defaultrocket (Math|Conversions|ToTransform(Vector) (Transformation|GetActorLocation)) "AlwaysSpawn" "MultiplyWithRoot" 0 0))
    (Utilities|IsValid _combat
      (:Is%20Valid
        (Class|CombatComponent|EquipWeapon _combat _returnvalue)))))

(event Custom|EquipSniper
  (bind _combat (Variables|Default|GetCombat))
  (bind _defaultsniper (Variables|Default|GetDefaultSniper))
  (if (Utilities|IsValidClass _defaultsniper)
    (bind _returnvalue (Game|SpawnActorfromClass _defaultsniper (Math|Conversions|ToTransform(Vector) (Transformation|GetActorLocation)) "AlwaysSpawn" "MultiplyWithRoot" 0 0))
    (Utilities|IsValid _combat
      (:Is%20Valid
        (Class|CombatComponent|EquipWeapon _combat _returnvalue)))))

(event Custom|EquipGrenade
  (bind _defaultgrenade (Variables|Default|GetDefaultGrenade))
  (bind _combat (Variables|Default|GetCombat))
  (if (Utilities|IsValidClass _defaultgrenade)
    (bind _returnvalue (Game|SpawnActorfromClass _defaultgrenade (Math|Conversions|ToTransform(Vector) (Transformation|GetActorLocation)) "AlwaysSpawn" "MultiplyWithRoot" 0 0))
    (Utilities|IsValid _combat
      (:Is%20Valid
        (Class|CombatComponent|EquipWeapon _combat _returnvalue)))))

(event EventBeginPlay
  (bind _self self)
  (bind _returnvalue (AI|GetAIController _self))
  (Utilities|FlowControl|Sequence
    (:then_0
      (bind _asbp_coop_game_mode (Utilities|Casting|CastToBP_CoopGameMode (Game|GetGameMode)))
      (Utilities|IsValid _asbp_coop_game_mode
        (:Is%20Valid
          (Class|CoopGameMode|AddSpawnedBotNum _asbp_coop_game_mode))))
    (:then_1
      (Utilities|IsValid _returnvalue
        (:Is%20Valid
          (AI|RunBehaviorTree _returnvalue "/Game/Blueprints/AI/AdvancedAI/BehaviorTree/BT_AdvancedAI.BT_AdvancedAI"))))))

(event EventDestroyed
  (bind _asbp_coop_game_mode (Utilities|Casting|CastToBP_CoopGameMode (Game|GetGameMode)))
  (Utilities|IsValid _asbp_coop_game_mode
    (:Is%20Valid
      (Class|CoopGameMode|SubSpawnedBotNum _asbp_coop_game_mode))))

(fn ConstructionScript)